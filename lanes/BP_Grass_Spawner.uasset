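; Spawner actor that lays down a chained row of BP_Grass lane segments when play begins.
; BeginPlay spawns 150 segments: the first at the spawner's location, each later one at the GrSpawnPoint of the newest segment.
; Each new segment becomes NewestGrLane and receives a reference back to this spawner.
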(event EventBeginPlay
  (CallFunction|SpawnInitialGrLanes))

(event Collision|EventActorBeginOverlap
  (params (OtherActor :type Actor%20Object%20Reference)))

(event EventTick
  (params (DeltaSeconds :type Float%20%28single-precision%29)))

(fn ConstructionScript)

(fn SpawnGrLanes
  (params (Gr_Spawn_Loc :type Vector))
  (bind _returnvalue (Game|SpawnActorfromClass "/Game/Terrains/BP_Grass.BP_Grass_C" (Math|Transform|MakeTransform Gr_Spawn_Loc "0, 0, 0" "1,1,1") "Undefined" 0 0))
  (bind _output_get (Variables|Default|SetNewest_GrLane _returnvalue))
  (Variables|/Game/Terrains/BP_Grass.BP_Grass_C|SetGrLane_Spawner _output_get self))

(fn SpawnGratSpawnPoint
  (CallFunction|SpawnGrLanes (Transformation|GetWorldLocation (Variables|/Game/Terrains/BP_Grass.BP_Grass_C|GetGrSpawnPoint (Variables|Default|GetNewest_GrLane)))))

(fn SpawnInitialGrLanes
  (for _index (range 0 149)
    (Utilities|IsValid (Variables|Default|GetNewest_GrLane)
      (:Is%20Valid
        (CallFunction|SpawnGratSpawnPoint))
      (:Is%20Not%20Valid
        (CallFunction|SpawnGrLanes (Transformation|GetActorLocation))))))