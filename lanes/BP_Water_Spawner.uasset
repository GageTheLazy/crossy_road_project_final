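; BP_Water_Spawner builds a continuous chain of BP_Water lane segments when play begins.
; The first segment spawns at the spawner's location, and each of the 150 iterations after that chains onto the WtSpawnPoint of the newest segment.
; Each spawned segment becomes NewestWater and receives a reference back to the spawner.
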(event EventBeginPlay
  (CallFunction|SpawnInitialWater))

(event Collision|EventActorBeginOverlap
  (params (OtherActor :type Actor%20Object%20Reference)))

(event EventTick
  (params (DeltaSeconds :type Float%20%28single-precision%29)))

(fn ConstructionScript)

(fn SpawnWtLanes
  (params (Wt_Spawn_Loc :type Vector))
  (bind _returnvalue (Game|SpawnActorfromClass "/Game/Terrains/BP_Water.BP_Water_C" (Math|Transform|MakeTransform Wt_Spawn_Loc "0, 0, 0" "1,1,1") "Undefined" 0 0))
  (bind _output_get (Variables|Default|SetNewest_Water _returnvalue))
  (Variables|/Game/Terrains/BP_Water.BP_Water_C|SetWt_Spawner _output_get self))

(fn SpawnWtatSpawnPoint
  (CallFunction|SpawnWtLanes (Transformation|GetWorldLocation (Variables|/Game/Terrains/BP_Water.BP_Water_C|GetWt_SpawnPoint (Variables|Default|GetNewest_Water)))))

(fn SpawnInitialWater
  (for _index (range 0 149)
    (Utilities|IsValid (Variables|Default|GetNewest_Water)
      (:Is%20Valid
        (CallFunction|SpawnWtatSpawnPoint))
      (:Is%20Not%20Valid
        (CallFunction|SpawnWtLanes (Transformation|GetActorLocation))))))