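; BP_Road_Spawner builds a chain of BP_Road segments when play begins, laying out the initial road.
; The first segment spawns at the spawner's location, and each later one at the newest road's RdSpawnPoint, for 150 in total.
; Each road receives a reference back to the spawner and becomes NewestRoad.
; SpawnCarOnLane is an empty stub with a disconnected SpawnCar call.
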(event EventBeginPlay
  (CallFunction|SpawnInitialRoads))

(event Collision|EventActorBeginOverlap
  (params (OtherActor :type Actor%20Object%20Reference)))

(event EventTick
  (params (DeltaSeconds :type Float%20%28single-precision%29)))

(fn ConstructionScript)

(fn SpawnRdLanes
  (params (Rd_Spawn_Loc :type Vector))
  (bind _returnvalue (Game|SpawnActorfromClass "/Game/Terrains/BP_Road.BP_Road_C" (Math|Transform|MakeTransform Rd_Spawn_Loc "0, 0, 0" "1,1,1") "Undefined" 0 0))
  (bind _output_get (Variables|Default|SetNewest%20Road _returnvalue))
  (Variables|/Game/Terrains/BP_Road.BP_Road_C|SetRd_Spawner _output_get self))

(fn SpawnRdatSpawnPoint
  (CallFunction|SpawnRdLanes (Transformation|GetWorldLocation (Variables|/Game/Terrains/BP_Road.BP_Road_C|GetRd_SpawnPoint (Variables|Default|GetNewest%20Road)))))

(fn SpawnInitialRoads
  (for _index (range 0 149)
    (Utilities|IsValid (Variables|Default|GetNewest%20Road)
      (:Is%20Valid
        (CallFunction|SpawnRdatSpawnPoint))
      (:Is%20Not%20Valid
        (CallFunction|SpawnRdLanes (Transformation|GetActorLocation))))))

(fn SpawnCaronLane)