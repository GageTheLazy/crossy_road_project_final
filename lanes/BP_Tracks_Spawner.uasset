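; BP_Tracks_Spawner builds a continuous chain of BP_Tracks lane segments in the level.
; On BeginPlay it spawns 150 segments, placing the first at its own location and each later one at the TxSpawnPoint of the newest segment.
; Each spawned segment becomes NewestTracks and receives a reference back to the spawner through its TxSpawner variable.
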(event EventBeginPlay
  (CallFunction|SpawnInitialTracks))

(event Collision|EventActorBeginOverlap
  (params (OtherActor :type Actor%20Object%20Reference)))

(event EventTick
  (params (DeltaSeconds :type Float%20%28single-precision%29)))

(fn ConstructionScript)

(fn SpawnTxLanes
  (params (Tx_Spawn_Loc :type Vector))
  (bind _returnvalue (Game|SpawnActorfromClass "/Game/Terrains/BP_Tracks.BP_Tracks_C" (Math|Transform|MakeTransform Tx_Spawn_Loc "0, 0, 0" "1,1,1") "Undefined" 0 0))
  (bind _output_get (Variables|Default|SetNewest_Tracks _returnvalue))
  (Variables|/Game/Terrains/BP_Tracks.BP_Tracks_C|SetTx_Spawner _output_get self))

(fn SpawnTxatSpawnPoint
  (CallFunction|SpawnTxLanes (Transformation|GetWorldLocation (Variables|/Game/Terrains/BP_Tracks.BP_Tracks_C|GetTx_SpawnPoint (Variables|Default|GetNewest_Tracks)))))

(fn SpawnInitialTracks
  (for _index (range 0 149)
    (Utilities|IsValid (Variables|Default|GetNewest_Tracks)
      (:Is%20Valid
        (CallFunction|SpawnTxatSpawnPoint))
      (:Is%20Not%20Valid
        (CallFunction|SpawnTxLanes (Transformation|GetActorLocation))))))