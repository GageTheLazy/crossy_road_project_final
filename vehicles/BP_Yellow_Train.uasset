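; BP_Yellow_Train is a moving train obstacle that kills the player on contact.
; Tick moves it by a swept local offset from its forward and lane speeds.
; When TrainTriggerZone overlaps another BP_Yellow_Train, TrainsSpawner spawns a train and this one destroys itself.
; When its mesh overlaps BP_Player, it plays a death sound, destroys the player and quits the game after a short delay.
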(event OnComponentBeginOverlap(TrainTriggerZone)
  (params (OverlappedComponent :type Primitive%20Component%20Object%20Reference) (OtherActor :type Actor%20Object%20Reference) (OtherComp :type Primitive%20Component%20Object%20Reference) (OtherBodyIndex :type Integer) (bFromSweep :type Boolean) (SweepResult :type Hit%20Result%20Structure%20%28by%20ref%29))
  (Utilities|Casting|CastToBP_Yellow_Train OtherActor)
  (Default|SpawnTrainatSpawnPoint (Variables|Default|GetTrains_Spawner))
  (Actor|DestroyActor))

(event OnComponentBeginOverlap(train_mesh)
  (params (OverlappedComponent :type Primitive%20Component%20Object%20Reference) (OtherActor :type Actor%20Object%20Reference) (OtherComp :type Primitive%20Component%20Object%20Reference) (OtherBodyIndex :type Integer) (bFromSweep :type Boolean) (SweepResult :type Hit%20Result%20Structure%20%28by%20ref%29))
  (bind _asbp_player (Utilities|Casting|CastToBP_Player OtherActor))
  (Audio|PlaySoundatLocation "/Game/Sounds/death_sound.death_sound" (Transformation|GetActorLocation _asbp_player) "0, 0, 0" 1.0 1.0 0.0 0 0 0)
  (Actor|DestroyActor _asbp_player)
  (Utilities|FlowControl|Delay 1.5)
  (Game|QuitGame 0 "Quit" false))

(event EventBeginPlay)

(event Collision|EventActorBeginOverlap
  (params (OtherActor :type Actor%20Object%20Reference)))

(event EventTick
  (params (DeltaSeconds :type Float%20%28single-precision%29))
  (Transformation|AddActorLocalOffset (Math|Vector|MakeVector (* DeltaSeconds (Variables|Default|Gettrain_speed)) (* (Variables|Default|Gettrain_lane_speed) DeltaSeconds) 0.0) true false))

(fn ConstructionScript)