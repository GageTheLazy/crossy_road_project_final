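; BP_Car_Spawner populates the level with a chain of BP_Blue_Car actors on BeginPlay.
; The first car spawns at the spawner's location and becomes NewestCar.
; Each later loop pass spawns one car at NewestCar's CarSpawnPoint, then another at that new car's CarSpawnPointLanes, over 150 passes total.
; Every car receives a CarSpawner reference back to this actor.
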(event EventBeginPlay
  (CallFunction|SpawnInitialCars))

(event Collision|EventActorBeginOverlap
  (params (OtherActor :type Actor%20Object%20Reference)))

(event EventTick
  (params (DeltaSeconds :type Float%20%28single-precision%29)))

(fn ConstructionScript)

(fn SpawnCar
  (params (Spawn_Loc :type Vector))
  (bind _returnvalue (Game|SpawnActorfromClass "/Game/Vehicles/Cars/BP_Blue_Car.BP_Blue_Car_C" (Math|Transform|MakeTransform Spawn_Loc "0, 0, 0" "1,1,1") "Undefined" 0 0))
  (bind _output_get (Variables|Default|SetNewest_Car _returnvalue))
  (Variables|/Game/Vehicles/Cars/BP_Blue_Car.BP_Blue_Car_C|SetCar_Spawner _output_get self))

(fn SpawnCaratSpawnPoint
  (CallFunction|SpawnCar (Transformation|GetWorldLocation (Variables|/Game/Vehicles/Cars/BP_Blue_Car.BP_Blue_Car_C|GetCarSpawnPoint (Variables|Default|GetNewest_Car)))))

(fn SpawnInitialCars
  (for _index (range 0 149)
    (Utilities|IsValid (Variables|Default|GetNewest_Car)
      (:Is%20Valid
        (CallFunction|SpawnCaratSpawnPoint)
        (CallFunction|SpawnCaronRoads))
      (:Is%20Not%20Valid
        (CallFunction|SpawnCar (Transformation|GetActorLocation))))))

(fn SpawnCaronRoads
  (CallFunction|SpawnCar (Transformation|GetWorldLocation (Variables|/Game/Vehicles/Cars/BP_Blue_Car.BP_Blue_Car_C|GetCarSpawnPointLanes (Variables|Default|GetNewest_Car)))))