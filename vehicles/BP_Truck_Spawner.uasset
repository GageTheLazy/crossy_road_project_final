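; Spawner actor that fills the level with a chain of red trucks when play begins.
; A fixed loop places the first truck at the spawner's location, then alternates between the newest truck's TruckSpawnPoint and TruckSpawnPointLanes components, adding two trucks per iteration.
; Each spawned truck becomes NewestTruck, anchoring the next spawn, and receives a reference back to the spawner.
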(event EventBeginPlay
  (CallFunction|SpawnInitialTrucks))

(event Collision|EventActorBeginOverlap
  (params (OtherActor :type Actor%20Object%20Reference)))

(event EventTick
  (params (DeltaSeconds :type Float%20%28single-precision%29)))

(fn ConstructionScript)

(fn SpawnTrucks
  (params (Truck_Spawn_Loc :type Vector))
  (bind _returnvalue (Game|SpawnActorfromClass "/Game/Vehicles/Trucks/BP_Red_Truck.BP_Red_Truck_C" (Math|Transform|MakeTransform Truck_Spawn_Loc "0, 0, 0" "1,1,1") "Undefined" 0 0))
  (bind _output_get (Variables|Default|SetNewest_Truck _returnvalue))
  (Variables|/Game/Vehicles/Trucks/BP_Red_Truck.BP_Red_Truck_C|SetTrucks_Spawner _output_get self))

(fn SpawnTruckatSpawnPoint
  (CallFunction|SpawnTrucks (Transformation|GetWorldLocation (Variables|/Game/Vehicles/Trucks/BP_Red_Truck.BP_Red_Truck_C|GetTruckSpawnPoint (Variables|Default|GetNewest_Truck)))))

(fn SpawnInitialTrucks
  (for _index (range 0 149)
    (Utilities|IsValid (Variables|Default|GetNewest_Truck)
      (:Is%20Valid
        (CallFunction|SpawnTruckatSpawnPoint)
        (CallFunction|SpawnTruckonLanes))
      (:Is%20Not%20Valid
        (CallFunction|SpawnTrucks (Transformation|GetActorLocation))))))

(fn SpawnTruckonLanes
  (CallFunction|SpawnTrucks (Transformation|GetWorldLocation (Variables|/Game/Vehicles/Trucks/BP_Red_Truck.BP_Red_Truck_C|GetTruckSpawnPointLanes (Variables|Default|GetNewest_Truck)))))