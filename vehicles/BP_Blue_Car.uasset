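; BP_Blue_Car is a traffic car that drives by a swept local offset each tick, using forward and lane speeds, and kills the chicken player on contact.
; When its CarTriggerZone overlaps a BP_Blue_Car, it asks CarSpawner for a new car and destroys itself.
; A mesh overlap with BP_Player squishes the skin, offsets it vertically, sets a Z plane-constraint normal, plays a death sound and quits the game after a delay.
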(event OnComponentBeginOverlap(CarTriggerZone)
  (params (OverlappedComponent :type Primitive%20Component%20Object%20Reference) (OtherActor :type Actor%20Object%20Reference) (OtherComp :type Primitive%20Component%20Object%20Reference) (OtherBodyIndex :type Integer) (bFromSweep :type Boolean) (SweepResult :type Hit%20Result%20Structure%20%28by%20ref%29))
  (Utilities|Casting|CastToBP_Blue_Car OtherActor)
  (Default|SpawnCaratSpawnPoint (Variables|Default|GetCar_Spawner))
  (Actor|DestroyActor))

(event OnComponentBeginOverlap(car_mesh)
  (params (OverlappedComponent :type Primitive%20Component%20Object%20Reference) (OtherActor :type Actor%20Object%20Reference) (OtherComp :type Primitive%20Component%20Object%20Reference) (OtherBodyIndex :type Integer) (bFromSweep :type Boolean) (SweepResult :type Hit%20Result%20Structure%20%28by%20ref%29))
  (bind _asbp_player (Utilities|Casting|CastToBP_Player OtherActor))
  (Transformation|SetWorldScale3D (Variables|/Game/BP_Player.BP_Player_C|GetChick_Skin _asbp_player) (Variables|/Game/BP_Player.BP_Player_C|Getchicken_squished _asbp_player))
  (Transformation|AddActorLocalOffset _asbp_player (Math|Vector|MakeVector 0.0 0.0 (+ (.z (Transformation|GetActorLocation (Game|GetPlayerCharacter 0))) -7e+02)) false false)
  (Class|MovementComponent|SetPlaneConstraintNormal (Variables|/Script/Engine.Character|GetCharacterMovement _asbp_player) (Math|Vector|MakeVector 0.0 0.0 1.0))
  (Audio|PlaySoundatLocation "/Game/Sounds/death_sound.death_sound" (Transformation|GetActorLocation _asbp_player) "0, 0, 0" 1.0 1.0 0.0 0 0 0)
  (Utilities|FlowControl|Delay 1.5)
  (Game|QuitGame 0 "Quit" false))

(event EventBeginPlay)

(event Collision|EventActorBeginOverlap
  (params (OtherActor :type Actor%20Object%20Reference)))

(event EventTick
  (params (DeltaSeconds :type Float%20%28single-precision%29))
  (Transformation|AddActorLocalOffset (Math|Vector|MakeVector (* DeltaSeconds (Variables|Default|Getcar_speed)) (* DeltaSeconds (Variables|Default|Getcar_lane_speed)) 0.0) true false))

(fn ConstructionScript)