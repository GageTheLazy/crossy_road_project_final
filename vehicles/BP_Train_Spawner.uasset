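; Spawner actor that lays out a chain of BP_Yellow_Train actors when play begins.
; A fixed loop seeds the first train at the spawner, then adds two per pass, each placed from the previous train's spawn point components.
; Placement alternates between TrainSpawnPoint and TrainSpawnPointLanes.
; Each new train becomes NewestTrain and receives a reference back to the spawner.
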(event EventBeginPlay
  (CallFunction|SpawnInitialTrains))

(event Collision|EventActorBeginOverlap
  (params (OtherActor :type Actor%20Object%20Reference)))

(event EventTick
  (params (DeltaSeconds :type Float%20%28single-precision%29)))

(fn ConstructionScript)

(fn SpawnTrains
  (params (Train_Spawn_Loc :type Vector))
  (bind _returnvalue (Game|SpawnActorfromClass "/Game/Vehicles/Trains/BP_Yellow_Train.BP_Yellow_Train_C" (Math|Transform|MakeTransform Train_Spawn_Loc "0, 0, 0" "1,1,1") "Undefined" 0 0))
  (bind _output_get (Variables|Default|SetNewest_Train _returnvalue))
  (Variables|/Game/Vehicles/Trains/BP_Yellow_Train.BP_Yellow_Train_C|SetTrains_Spawner _output_get self))

(fn SpawnTrainatSpawnPoint
  (CallFunction|SpawnTrains (Transformation|GetWorldLocation (Variables|/Game/Vehicles/Trains/BP_Yellow_Train.BP_Yellow_Train_C|GetTrainSpawnPoint (Variables|Default|GetNewest_Train)))))

(fn SpawnInitialTrains
  (for _index (range 0 149)
    (Utilities|IsValid (Variables|Default|GetNewest_Train)
      (:Is%20Valid
        (CallFunction|SpawnTrainatSpawnPoint)
        (CallFunction|SpawnTrainonLanes))
      (:Is%20Not%20Valid
        (CallFunction|SpawnTrains (Transformation|GetActorLocation))))))

(fn SpawnTrainonLanes
  (CallFunction|SpawnTrains (Transformation|GetWorldLocation (Variables|/Game/Vehicles/Trains/BP_Yellow_Train.BP_Yellow_Train_C|GetTrainSpawnPointLanes (Variables|Default|GetNewest_Train)))))