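; BP_Player is a player character Blueprint handling walking, strafing, jumping and a few sound cues.
; Movement axes follow control-rotation yaw only, JumpUp triggers Jump, and UpButton plays a one-shot walk sound at the player's location.
; BeginPlay checks once whether the character is falling; if so, it plays an eagle sound and quits the game after a short delay.
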(event EventBeginPlay
  (if (AI|Components|NavMovement|IsFalling (Variables|Character|GetCharacterMovement))
    (Audio|PlaySoundatLocation "/Game/Sounds/eagle_sound.eagle_sound" (Transformation|GetActorLocation) "0, 0, 0" 1.0 1.0 0.0 0 0 0)
    (Utilities|FlowControl|Delay 2.0)
    (Game|QuitGame 0 "Quit" false)))

(event Collision|EventActorBeginOverlap
  (params (OtherActor :type Actor%20Object%20Reference)))

(event EventTick
  (params (DeltaSeconds :type Float%20%28single-precision%29)))

(event Input|ActionEvents|InputActionJumpUp
  (params (Key :type Key%20Structure :default "None"))
  (:Pressed
    (Character|Jump)))

(event Input|ActionEvents|InputActionUpButton
  (params (Key :type Key%20Structure :default "None"))
  (:Pressed
    (Audio|PlaySoundatLocation "/Game/Sounds/walk_sound.walk_sound" (Transformation|GetActorLocation) "0, 0, 0" 1.0 1.0 0.0 0 0 0)))

(event Input|AxisEvents|InputAxisWalkMovement
  (params (AxisValue :type Float%20%28single-precision%29))
  (Pawn|Input|AddMovementInput (Math|Vector|GetForwardVector (Math|Rotator|MakeRotator 0.0 0.0 (.Yaw (Math|Rotator|BreakRotator (Pawn|GetControlRotation :!class /Script/Engine.Pawn))))) AxisValue false))

(event Input|AxisEvents|InputAxisSideStep
  (params (AxisValue :type Float%20%28single-precision%29))
  (Pawn|Input|AddMovementInput (Math|Vector|GetRightVector (Math|Rotator|MakeRotator 0.0 0.0 (.Yaw (Math|Rotator|BreakRotator (Pawn|GetControlRotation :!class /Script/Engine.Pawn))))) AxisValue false))

(fn ConstructionScript)